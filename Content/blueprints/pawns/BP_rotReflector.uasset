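; BP_rotReflector is a pawn, by its name a rotatable reflector, whose mesh is pushed and rotated by player input.
; While the "test" axis reads 1, it applies a large physics force to the mesh along the follow camera's forward vector.
; While the "space" axis reads 1, it rotates the mesh in world space by a fixed step per axis event.
; A debug print of MatValForScan is left unconnected.
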(event EventBeginPlay)

(event Collision|EventActorBeginOverlap
  (params (OtherActor :type Actor%20Object%20Reference)))

(event EventTick
  (params (DeltaSeconds :type Float%20%28single-precision%29)))

(event Input|AxisEvents|InputAxistest
  (params (AxisValue :type Float%20%28single-precision%29))
  (if (== AxisValue 1.0)
    (Physics|AddForce (Variables|Character|GetMesh) (* (Math|Vector|GetForwardVector (Variables|Default|GetFollowCamera)) 9e+04) "None" false)))

(event Input|AxisEvents|InputAxisspace
  (params (AxisValue :type Float%20%28single-precision%29))
  (if (== AxisValue 1.0)
    (Transformation|AddWorldRotation (Variables|Character|GetMesh) "0,1.000000, 0" false false)))

(fn ConstructionScript)