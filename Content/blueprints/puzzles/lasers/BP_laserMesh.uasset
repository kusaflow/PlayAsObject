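; BP_laserMesh is a puzzle laser actor that draws a beam as a stretched mesh between two points.
; Its LaserMeshProj event places Lmesh at Start and aligns its Z axis to the Start-End direction.
; It scales width by LaserThickness and length by distance over 100, negating Z so the mesh reaches toward End.
; Construction script, BeginPlay and Tick are empty, so callers drive all updates through that event.
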(event EventBeginPlay)

(event Collision|EventActorBeginOverlap
  (params (OtherActor :type Actor%20Object%20Reference)))

(event EventTick
  (params (DeltaSeconds :type Float%20%28single-precision%29)))

(event EventLaserMeshProj
  (params (start :type Vector :default "0, 0, 0") (end :type Vector :default "0, 0, 0"))
  (bind _returnvalue (- start end))
  (bind _lmesh (Variables|Default|GetLmesh))
  (bind _laserthickness (Variables|Default|GetLaserThickness))
  (Transformation|SetWorldLocationAndRotation _lmesh start (Math|Rotator|MakeRotfromZ (Math|Vector|Normalize _returnvalue)) false true)
  (Transformation|SetWorldScale3D _lmesh (Math|Vector|MakeVector _laserthickness _laserthickness (* (/ (Math|Vector|VectorLength _returnvalue) 1e+02) -1.0))))

(fn ConstructionScript)