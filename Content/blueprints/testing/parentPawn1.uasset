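; Test pawn that orbits a spring arm camera, pushes its mesh with physics force and lets the player swap possession to another pawn.
; Axis inputs yaw the spring arm and adjust its clamped pitch, while a test axis accelerates the mesh along the camera's forward vector.
; On changePawn, the current player pawn line-traces from the camera and its controller possesses any parentPawn hit.
; BeginPlay enables custom depth rendering on the mesh.
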(event EventBeginPlay
  (Rendering|SetRenderCustomDepth (Variables|Default|GetStaticMesh) true))

(event Collision|EventActorBeginOverlap
  (params (OtherActor :type Actor%20Object%20Reference)))

(event Input|ActionEvents|InputActionchangePawn
  (params (Key :type Key%20Structure :default "None"))
  (bind _camera (Variables|Default|GetCamera))
  (bind _returnvalue (Transformation|GetWorldLocation _camera))
  (:Pressed
    (if (== self (Game|Player|GetPlayerPawn 0))
      (bind _outhit (Collision|LineTraceByChannel _returnvalue (+ _returnvalue (* (Math|Vector|GetForwardVector _camera) 2e+03)) "TraceTypeQuery1" false 0 "ForOneFrame"))
      (bind _asparent_pawn (Utilities|Casting|CastToparentPawn (.hitactor _outhit)))
      (Pawn|Possess (Pawn|GetController) _asparent_pawn))))

(event Input|AxisEvents|InputAxisxAxis
  (params (AxisValue :type Float%20%28single-precision%29))
  (Transformation|AddRelativeRotation (Variables|Default|GetSpringArm) (Math|Rotator|MakeRotator 0.0 0.0 AxisValue) false false))

(event Input|AxisEvents|InputAxisyAxis
  (params (AxisValue :type Float%20%28single-precision%29))
  (bind _springarm (Variables|Default|GetSpringArm))
  (bind _relativerotation (Variables|/Script/Engine.SceneComponent|GetRelativeRotation _springarm))
  (Transformation|SetRelativeRotation _springarm (Math|Rotator|MakeRotator (.roll _relativerotation) (Math|Float|Clamp(Float) (+ AxisValue (.pitch _relativerotation)) -8e+01 4.0) (.yaw _relativerotation)) false false))

(event Input|AxisEvents|InputAxistest
  (params (AxisValue :type Float%20%28single-precision%29))
  (if (== AxisValue 1.0)
    (Physics|AddForce (Variables|Default|GetStaticMesh) (* (Math|Vector|GetForwardVector (Variables|Default|GetCamera)) 1e+03) "None" true)))

(fn ConstructionScript)